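; BP_CameraPawn is a sandbox camera pawn that can spawn a BP_Player creature and follow it or detach from it.
; While locked, Tick smoothly interpolates the pawn's location toward the controlled creature.
; Spring arm functions provide clamped zoom and pitch.
; Helpers toggle the lock, bind to a camera-lock widget's dispatcher, show or hide the action mesh, and give the spawned creature its default controller.
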(event `self.ReceiveBeginPlay`)

(event `self.ReceiveTick`
  (params (DeltaSeconds :type "Float (single-precision)"))
  (if (`self.bLockCamera`)
    (`self.K2_SetActorLocation` (`KismetMathLibrary.VInterpTo` (`self.K2_GetActorLocation`) (`self.K2_GetActorLocation` (`self.ControlledCreature`)) (`GameplayStatics.GetWorldDeltaSeconds`) 5.0) false true)))

(fn `AttachCamera`
  (set `self.bLockCamera` true))

(fn `BindCameraLock`
  (params (CameraLockWidget :type "/Game/Sandbox/UI/WBP_CameraLock Object Reference"))
  (add `/Game/Sandbox/UI/WBP_CameraLock.OnLockCamera_Disp` CameraLockWidget (`|CreateDelegate` :!event `CameraLock`)))

(fn `Camera Pitch Rotate`
  (params (InVal :type "Float (double-precision)"))
  (bind (_relativerotation_roll _relativerotation_pitch) (`KismetMathLibrary.BreakRotator` (`SceneComponent.RelativeRotation` (`self.SpringArm`))))
  (`SceneComponent.K2_SetRelativeRotation` (`self.SpringArm`) (`KismetMathLibrary.MakeRotator` 0.0 (`KismetMathLibrary.FClamp` (+ _relativerotation_pitch (* InVal (`GameplayStatics.GetWorldDeltaSeconds`) -90.0)) -80.0 -10.0)) false false))

(fn `CameraLock`
  (params (bCameraLock :type Boolean))
  (if bCameraLock
    (`self.AttachCamera`)
    (else
      (`self.DetachCamera`))))

(fn `CameraZoom`
  (params (Zoom :type "Float (double-precision)"))
  (bind _springarm (`self.SpringArm`))
  (set `SpringArmComponent.TargetArmLength` (`KismetMathLibrary.FClamp` (+ (* Zoom 100.0) (`SpringArmComponent.TargetArmLength` _springarm)) 300.0 5000.0) _springarm))

(fn `DetachCamera`
  (set `self.bLockCamera` false))

(fn `SetVisibilityActionMesh`
  (params (bNewVisibility :type Boolean))
  (`SceneComponent.SetVisibility` (`self.ActionMesh`) bNewVisibility false))

(fn `Spawn Creature`
  (bind _returnvalue (`|SpawnActorFromClass` "/Game/Sandbox/Blueprints/BP_Player.BP_Player_C" (`KismetMathLibrary.MakeTransform` (`self.K2_GetActorLocation`)) "AlwaysSpawn" "MultiplyWithRoot" null null))
  (bind _output_get (set `self.ControlledCreature` _returnvalue))
  (`self.SpawnDefaultController` _output_get))

(fn `UserConstructionScript`)