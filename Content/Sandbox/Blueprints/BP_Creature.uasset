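; BP_Creature is a sandbox creature Blueprint with a skeletal mesh, a body component, a team and attack-direction tags.
; On construction and BeginPlay it tints a dynamic body material by team as a debug aid.
; Helper functions bind an attack-direction widget's change event, add or remove direction tags, and expose the body component and bone names.
; An unconnected graph fragment holds a partial-ragdoll setup for the right arm.
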(event `self.ReceiveBeginPlay`
  (`self.TeamColor_DEBUG`))

(fn `BindChangeAttackDirection`
  (params (AttackDirectionWidget :type "/Game/Sandbox/UI/WBP_AttackDirection Object Reference"))
  (add `/Game/Sandbox/UI/WBP_AttackDirection.OnChangedAttackDirection_Disp` AttackDirectionWidget (`|CreateDelegate` :!event `ChangeAttackDirection`)))

(fn `ChangeAttackDirection`
  (params (bChecked :type Boolean) (Tag :type "GameplayTag Structure"))
  (if bChecked
    (`self.AddAttackDirectionTag` Tag)
    (else
      (`self.RemoveAttackDirectionTag` Tag))))

(fn `GetBodyComponent`
  (returns (BodyComponent :type "BodyComponent Object Reference"))
  (return (`self.BodyComponent`)))

(fn `GetBoneNames`
  (returns (Result :type "Array of Name"))
  (locals (L_Result :type "Array of Name"))
  (for _index (range (+ (`SkinnedMeshComponent.GetNumBones` (`self.Mesh`)) 1))
    (`KismetArrayLibrary.Array_Add` (`local.L_Result`) (`SkinnedMeshComponent.GetBoneName` (`self.Mesh`) _index)))
  (return (`local.L_Result`)))

(fn `TeamColor_DEBUG`
  (bind _returnvalue (`PrimitiveComponent.CreateDynamicMaterialInstance` (`self.Mesh`) 0 "/Game/Mannequin/Character/Materials/M_UE4Man_Body.M_UE4Man_Body" "None"))
  (switch `ETeam` (`self.GetTeam`)
    (:`Player`
      (`MaterialInstanceDynamic.SetVectorParameterValue` _returnvalue "BodyColor" (struct :`R` 0.450786 :`G` 0.401978 :`B` 0.361307 :`A` 1.0)))
    (:`Red`
      (`MaterialInstanceDynamic.SetVectorParameterValue` _returnvalue "BodyColor" (struct :`R` 0.863157 :`G` 0.06301 :`B` 0.06301 :`A` 1.0)))
    (:`Green`
      (`MaterialInstanceDynamic.SetVectorParameterValue` _returnvalue "BodyColor" (struct :`R` 0.06301 :`G` 0.863157 :`B` 0.06301 :`A` 1.0)))
    (:`Blue`
      (`MaterialInstanceDynamic.SetVectorParameterValue` _returnvalue "BodyColor" (struct :`R` 0.06301 :`G` 0.06301 :`B` 0.863157 :`A` 1.0)))
    (:`Yellow`
      (`MaterialInstanceDynamic.SetVectorParameterValue` _returnvalue "BodyColor" (struct :`R` 0.863157 :`G` 0.863157 :`B` 0.06301 :`A` 1.0)))))

(fn `UserConstructionScript`
  (`self.TeamColor_DEBUG`))