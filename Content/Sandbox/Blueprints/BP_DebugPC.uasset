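; Debug player controller for click-to-command play of an AI-driven creature through a free camera pawn.
; On possess, it has the camera spawn the creature, binds the debug HUD to it, and blocks click commands on unconsciousness or death.
; Enhanced Input drives camera pan, rotation and zoom.
; Clicks trigger GameplayInterface targets or set Shift-queueable destinations, while stop/continue inputs send gameplay tags, both via the creature's AI controller.
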(event `OnUpdateConsciousDelegate`
  (params (bIsUnconscious :type Boolean))
  (set `self.bCanMovementControlledPawn` (not bIsUnconscious)))

(event `self.ReceivePossess`
  (params (PossessedPawn :type "Pawn Object Reference"))
  (bind _controlledcreature (`/Game/Sandbox/Blueprints/BP_CameraPawn.ControlledCreature` (`self.ControlledCamera`)))
  (bind _asbp_camera_pawn (cast `/Game/Sandbox/Blueprints/BP_CameraPawn` PossessedPawn))
  (bind _output_get (set `self.ControlledCamera` _asbp_camera_pawn))
  (`/Game/Sandbox/Blueprints/BP_CameraPawn.Spawn Creature` _output_get)
  (bind _controlledcreature_2 (`/Game/Sandbox/Blueprints/BP_CameraPawn.ControlledCreature` _output_get))
  (bind _returnvalue (`|CreateWidget` "/Game/Sandbox/UI/WBP_DebugHUD.WBP_DebugHUD_C" self (`/Game/Sandbox/Blueprints/BP_Creature.GetBodyComponent` _controlledcreature_2) (`CreatureCore.AttributesComponent` _controlledcreature_2) (`CreatureCore.InventoryComponent` _controlledcreature_2) (`CreatureCore.EquipmentComponent` _controlledcreature_2)))
  (bind _output_get_2 (set `self.DebugHUD` _returnvalue))
  (`UserWidget.AddToViewport` _output_get_2 0)
  (`/Game/Sandbox/Blueprints/BP_Creature.BindChangeAttackDirection` (`/Game/Sandbox/Blueprints/BP_CameraPawn.ControlledCreature` (`self.ControlledCamera`)) (`/Game/Sandbox/UI/WBP_DebugHUD.WBP_AttackDirection` _output_get_2))
  (`/Game/Sandbox/Blueprints/BP_CameraPawn.BindCameraLock` (`self.ControlledCamera`) (`/Game/Sandbox/UI/WBP_DebugHUD.WBP_CameraLock` _output_get_2))
  (`|ExecutionSequence`
    (:`then_0`
      (add `CreatureCore.OnUpdateConsciousDelegate` _controlledcreature (delegate `OnUpdateConsciousDelegate`)))
    (:`then_1`
      (add `BodyComponent.OnDeathDelegate` (`/Game/Sandbox/Blueprints/BP_Creature.GetBodyComponent` _controlledcreature) (delegate `OnUnconsciousDelegate`)))))

(event `OnUnconsciousDelegate`
  (set `self.bCanMovementControlledPawn` false))

(event `self.ReceiveBeginPlay`
  (`EnhancedInputSubsystemInterface.AddMappingContext` (subsystem `EnhancedInputLocalPlayerSubsystem`) "/Game/Sandbox/Inputs/IMC_Default.IMC_Default" 0 (struct))
  (`WidgetBlueprintLibrary.SetInputMode_GameAndUIEx` self null "DoNotLock" false true))

(event `EnhancedInput|/Game/Sandbox/Inputs/IA_MouseMove`
  (params (ActionValue :type "Vector2D Structure") (ElapsedSeconds :type "Float (double-precision)") (TriggeredSeconds :type "Float (double-precision)") (InputAction :type "InputAction Object Reference" :default "/Game/Sandbox/Inputs/IA_MouseMove.IA_MouseMove"))
  (bind (_x _y) (`KismetMathLibrary.BreakVector2D` ActionValue))
  (bind _returnvalue (`GameplayStatics.GetWorldDeltaSeconds`))
  (bind _cameraspeed (`self.CameraSpeed`))
  (bind _controlledcamera (`self.ControlledCamera`))
  (bind _controlledcamera_2 (`self.ControlledCamera`))
  (:`Triggered`
    (`|ExecutionSequence`
      (:`then_0`
        (if (`self.bCanMoveCamera`)
          (`self.K2_AddActorWorldOffset` _controlledcamera (+ (* (`self.GetActorForwardVector` _controlledcamera) (* _x _cameraspeed _returnvalue)) (* (`self.GetActorRightVector` _controlledcamera) (* _y _cameraspeed _returnvalue))) false true)))
      (:`then_1`
        (if (`self.bCanRotateCamera`)
          (`self.K2_AddActorWorldRotation` _controlledcamera_2 (`KismetMathLibrary.MakeRotator` 0.0 0.0 (* _y _returnvalue 360.0)) false false)
          (`/Game/Sandbox/Blueprints/BP_CameraPawn.Camera Pitch Rotate` _controlledcamera_2 _x))))))

(event `EnhancedInput|/Game/Sandbox/Inputs/IA_RMB`
  (params (ActionValue :type Boolean) (ElapsedSeconds :type "Float (double-precision)") (TriggeredSeconds :type "Float (double-precision)") (InputAction :type "InputAction Object Reference" :default "/Game/Sandbox/Inputs/IA_RMB.IA_RMB"))
  (bind _controlledcamera (`self.ControlledCamera`))
  (:`Started`
    (set `self.bCanMoveCamera` true)
    (`/Game/Sandbox/Blueprints/BP_CameraPawn.SetVisibilityActionMesh` _controlledcamera true))
  (:`Completed`
    (set `self.bCanMoveCamera` false)
    (`/Game/Sandbox/Blueprints/BP_CameraPawn.SetVisibilityActionMesh` _controlledcamera false)))

(event `EnhancedInput|/Game/Sandbox/Inputs/IA_StopMove`
  (params (ActionValue :type Boolean) (ElapsedSeconds :type "Float (double-precision)") (TriggeredSeconds :type "Float (double-precision)") (InputAction :type "InputAction Object Reference" :default "/Game/Sandbox/Inputs/IA_StopMove.IA_StopMove"))
  (bind _returnvalue (`AIBlueprintHelperLibrary.GetAIController` (`/Game/Sandbox/Blueprints/BP_CameraPawn.ControlledCreature` (`self.ControlledCamera`))))
  (:`Started`
    (if (`KismetSystemLibrary.DoesImplementInterface` _returnvalue "/Script/Sandbox_Prototype.AIHelperInterface")
      (message `AIHelperInterface.SetAINewActionTag` _returnvalue (`BlueprintGameplayTagLibrary.MakeLiteralGameplayTag` (struct :`TagName` "Creature.Action.Idle"))))))

(event `EnhancedInput|/Game/Sandbox/Inputs/IA_MMB`
  (params (ActionValue :type Boolean) (ElapsedSeconds :type "Float (double-precision)") (TriggeredSeconds :type "Float (double-precision)") (InputAction :type "InputAction Object Reference" :default "/Game/Sandbox/Inputs/IA_MMB.IA_MMB"))
  (bind _controlledcamera (`self.ControlledCamera`))
  (:`Started`
    (set `self.bCanRotateCamera` true)
    (`/Game/Sandbox/Blueprints/BP_CameraPawn.SetVisibilityActionMesh` _controlledcamera true))
  (:`Completed`
    (set `self.bCanRotateCamera` false)
    (`/Game/Sandbox/Blueprints/BP_CameraPawn.SetVisibilityActionMesh` _controlledcamera false)))

(event `EnhancedInput|/Game/Sandbox/Inputs/IA_ContinueMove`
  (params (ActionValue :type Boolean) (ElapsedSeconds :type "Float (double-precision)") (TriggeredSeconds :type "Float (double-precision)") (InputAction :type "InputAction Object Reference" :default "/Game/Sandbox/Inputs/IA_ContinueMove.IA_ContinueMove"))
  (bind _returnvalue (`AIBlueprintHelperLibrary.GetAIController` (`/Game/Sandbox/Blueprints/BP_CameraPawn.ControlledCreature` (`self.ControlledCamera`))))
  (:`Triggered`
    (if (`KismetSystemLibrary.DoesImplementInterface` _returnvalue "/Script/Sandbox_Prototype.AIHelperInterface")
      (message `AIHelperInterface.SetAINewActionTag` _returnvalue (`BlueprintGameplayTagLibrary.MakeLiteralGameplayTag` (struct :`TagName` "Creature.Action.Move"))))))

(event `EnhancedInput|/Game/Sandbox/Inputs/IA_MouseWheel`
  (params (ActionValue :type "Float (double-precision)") (ElapsedSeconds :type "Float (double-precision)") (TriggeredSeconds :type "Float (double-precision)") (InputAction :type "InputAction Object Reference" :default "/Game/Sandbox/Inputs/IA_MouseWheel.IA_MouseWheel"))
  (:`Triggered`
    (`/Game/Sandbox/Blueprints/BP_CameraPawn.CameraZoom` (`self.ControlledCamera`) ActionValue)))

(event `EnhancedInput|/Game/Sandbox/Inputs/IA_LMB`
  (params (ActionValue :type Boolean) (ElapsedSeconds :type "Float (double-precision)") (TriggeredSeconds :type "Float (double-precision)") (InputAction :type "InputAction Object Reference" :default "/Game/Sandbox/Inputs/IA_LMB.IA_LMB"))
  (bind (_hitresult _returnvalue) (`self.GetHitResultUnderCursorForObjects` (`|MakeArray` "ObjectTypeQuery1" "ObjectTypeQuery2" "ObjectTypeQuery8" "ObjectTypeQuery7" :!type "EObjectTypeQuery Enum")))
  (bind (_bblockinghit _binitialoverlap _time _distance _location _impactpoint _normal _impactnormal _physmat _hitactor) (`GameplayStatics.BreakHitResult` _hitresult))
  (bind _returnvalue_2 (`AIBlueprintHelperLibrary.GetAIController` (`/Game/Sandbox/Blueprints/BP_CameraPawn.ControlledCreature` (`self.ControlledCamera`))))
  (:`Started`
    (if (`self.bCanMovementControlledPawn`)
      (if _returnvalue
        (`KismetSystemLibrary.DrawDebugSphere` _impactpoint 20.0 8 (struct :`R` 0.046794 :`G` 1.0 :`A` 1.0) 5.0 2.0)
        (if (!= _hitactor (`/Game/Sandbox/Blueprints/BP_CameraPawn.ControlledCreature` (`self.ControlledCamera`)))
          (bind _bsuccess (`self.ChooseAction` _hitactor))
          (if _bsuccess
            _
            (elif (`KismetSystemLibrary.DoesImplementInterface` _returnvalue_2 "/Script/Sandbox_Prototype.AIHelperInterface")
              (if (`self.bShift`)
                (message `AIHelperInterface.AddTargetLocation` _returnvalue_2 _impactpoint)
                (else
                  (message `AIHelperInterface.SetTargetLocation` _returnvalue_2 _impactpoint))))))))))

(event `EnhancedInput|/Game/Sandbox/Inputs/IA_Shift`
  (params (ActionValue :type Boolean) (ElapsedSeconds :type "Float (double-precision)") (TriggeredSeconds :type "Float (double-precision)") (InputAction :type "InputAction Object Reference" :default "/Game/Sandbox/Inputs/IA_Shift.IA_Shift"))
  (:`Started`
    (set `self.bShift` true))
  (:`Completed`
    (set `self.bShift` false)))

(fn `ChooseAction`
  (params (HitActor :type "Actor Object Reference"))
  (returns (bSuccess :type Boolean))
  (bind _returnvalue (`self.GetComponentByClass` (`local.HitActor`) "/Game/Sandbox/Blueprints/BPC_Body.BPC_Body_C"))
  (if (`KismetSystemLibrary.DoesImplementInterface` HitActor "/Script/Sandbox_Prototype.GameplayInterface")
    (`|ExecutionSequence`
      (:`then_0`
        (message `GameplayInterface.Click` (`local.HitActor`) (`AIBlueprintHelperLibrary.GetAIController` (`/Game/Sandbox/Blueprints/BP_CameraPawn.ControlledCreature` (`self.ControlledCamera`))))
        (`/Engine/EditorBlueprintResources/StandardMacros.IsValid` _returnvalue
          (:`Is Valid`
            (`/Game/Sandbox/UI/WBP_DebugHUD.InitEnemyHealth` (`self.DebugHUD`) _returnvalue))))
      (:`then_1`
        (return true)))
    (else
      (return false))))

(fn `UserConstructionScript`)