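; BP_Enemy is an enemy Blueprint that gives itself a weapon shortly after spawning, through a debug equip routine.
; After a short BeginPlay delay, it reads the item list from BP_RPGGameInstance and builds weapon item objects from type-matching entries.
; It tries each in a fixed EquipmentComponent slot and stops at the first success, so despite the routine's name nothing is randomized.
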(event `self.ReceiveBeginPlay`
  (`parent.ReceiveBeginPlay`)
  (`KismetSystemLibrary.Delay` 2.0)
  (`self.EquipRandWeapon_DEBUG`))

(fn `EquipRandWeapon_DEBUG`
  (locals (L_Items :type "Array of RPGItemData Object Reference"))
  (bind _asbp_rpggame_instance (cast `/Game/Sandbox/Game/BP_RPGGameInstance` (`GameplayStatics.GetGameInstance`)))
  (bind _output_get (set `local.L_Items` (`/Game/Sandbox/Game/BP_RPGGameInstance.Items` _asbp_rpggame_instance)))
  (for _array_element _output_get
    (bind _commondata (`RPGItemData.CommonData` _array_element))
    (if (== (`.Type` (break `RPGItemInfo` _commondata)) "Weapon")
      (bind _returnvalue (`|GenericCreateObject` "/Script/Sandbox_Prototype.RPGItemObject_Weapon" (`RPGItemData_Weapon.WeaponInfo` (cast `RPGItemData_Weapon` _array_element :!pure true)) _commondata))
      (bind _returnvalue_2 (`EquipmentComponent.TryEquipItemByIndex` (`self.EquipmentComponent`) _returnvalue 4))
      (if _returnvalue_2
        (break)))))

(fn `UserConstructionScript`
  (`parent.UserConstructionScript`))