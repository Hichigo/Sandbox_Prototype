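; Sandbox player Blueprint for an RPG, with debug routines that exercise attribute progression and inventory.
; From BeginPlay, a fast looping timer grants experience to a random core attribute through the AttributesComponent.
; After a short delay, FillItemsDEBUG picks random item data from BP_RPGGameInstance and constructs generic or weapon item objects by type.
; Each object goes to the InventoryComponent, or is dropped if it cannot be added.
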(event `CustomEvent`
  (`AttributesComponent.ApplyAttributeExp` (`self.AttributesComponent`) (`KismetArrayLibrary.Array_Random` (`|MakeArray` (struct :`TagName` "Creature.Attribute.Type.Health") (struct :`TagName` "Creature.Attribute.Type.Strength") (struct :`TagName` "Creature.Attribute.Type.Agility") (struct :`TagName` "Creature.Attribute.Type.Intelligence") :!type "GameplayTag Structure")) 50.0))

(event `self.ReceiveBeginPlay`
  (`parent.ReceiveBeginPlay`)
  (`|ExecutionSequence`
    (:`then_0`
      (`KismetSystemLibrary.K2_SetTimerDelegate` (delegate `CustomEvent`) 0.1 true)
      (`KismetSystemLibrary.Delay` 1.0)
      (`self.FillItems_DEBUG`))))

(event `self.ReceiveTick`
  (params (DeltaSeconds :type "Float (single-precision)"))
  (`parent.ReceiveTick` DeltaSeconds))

(fn `FillItems_DEBUG`
  (locals (L_Items :type "Array of RPGItemData Object Reference") (L_CurrentItem :type "RPGItemData Object Reference"))
  (bind _commondata (`RPGItemData.CommonData` (`local.L_CurrentItem`)))
  (bind _type (break `RPGItemInfo` _commondata))
  (bind _asbp_rpggame_instance (cast `/Game/Sandbox/Game/BP_RPGGameInstance` (`GameplayStatics.GetGameInstance`)))
  (set `local.L_Items` (`/Game/Sandbox/Game/BP_RPGGameInstance.Items` _asbp_rpggame_instance))
  (for _ (range 41)
    (set `local.L_CurrentItem` (`KismetArrayLibrary.Array_Random` (`local.L_Items`)))
    (if (== _type "Item")
      (bind _returnvalue (`|GenericCreateObject` "/Script/Sandbox_Prototype.RPGItemObject" _commondata))
      (bind _returnvalue_2 (`InventoryComponent.TryAddItem` (`self.InventoryComponent`) _returnvalue))
      (if (not _returnvalue_2)
        (`RPGHelperFunctionLibrary.DropItem` _returnvalue self))
      (elif (== _type "Weapon")
        (bind _returnvalue_3 (`|GenericCreateObject` "/Script/Sandbox_Prototype.RPGItemObject_Weapon" (`RPGItemData_Weapon.WeaponInfo` (cast `RPGItemData_Weapon` (`local.L_CurrentItem`) :!pure true)) _commondata))
        (bind _returnvalue_4 (`InventoryComponent.TryAddItem` (`self.InventoryComponent`) _returnvalue_3))
        (if (not _returnvalue_4)
          (`RPGHelperFunctionLibrary.DropItem` _returnvalue_3 self))))))

(fn `UserConstructionScript`
  (`parent.UserConstructionScript`))