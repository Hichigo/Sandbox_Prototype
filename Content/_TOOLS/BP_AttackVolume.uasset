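; BP_AttackVolume is a tool volume that periodically damages creatures standing inside it.
; From BeginPlay, a looping one-second timer finds BP_Creature actors overlapping the Box and sends each a damage message with a random amount within Min/Max and a damage type tag.
; The construction script labels the TextRender from AttackBodyPartTag, but damage ignores that tag and always uses the "head" bone.
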(event `self.ReceiveBeginPlay`
  (`KismetSystemLibrary.K2_SetTimerDelegate` (delegate `OnMakeDamage`) 1.0 true))

(event `OnMakeDamage`
  (for _array_element (`PrimitiveComponent.GetOverlappingActors` (`self.Box`) "/Game/Sandbox/Blueprints/BP_Creature.BP_Creature_C")
    (message `DamageInterface.ReceiveDamage` _array_element (make `DamageInfo` (`KismetMathLibrary.RandomFloatInRange` (`self.MinDamage`) (`self.MaxDamage`)) "head" (`self.DamageTypeTag`) self))))

(fn `SetText`
  (params (BodyPartName :type Text))
  (`TextRenderComponent.K2_SetText` (`self.TextRender`) BodyPartName))

(fn `UserConstructionScript`
  (`|SwitchGameplayTag` (`self.AttackBodyPartTag`)
    (:`Default`
      (`self.SetText` "Random"))
    (:`BodyParts.All`
      (`self.SetText` "All"))
    (:`BodyParts.Main.Head`
      (`self.SetText` "Head"))
    (:`BodyParts.Main.Body`
      (`self.SetText` "Body"))
    (:`BodyParts.Secondary.Left.Hand`
      (`self.SetText` "Left hand"))
    (:`BodyParts.Secondary.Left.Leg`
      (`self.SetText` "Left leg"))
    (:`BodyParts.Secondary.Right.Hand`
      (`self.SetText` "Right hand"))
    (:`BodyParts.Secondary.Right.Leg`
      (`self.SetText` "Right leg"))))